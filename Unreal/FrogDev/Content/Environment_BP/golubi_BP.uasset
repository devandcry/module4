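; Pigeon flock obstacle ("golubi") that takes off once and hides when its flipbook animation ends, timed from frame count and rate.
; Touching Box while the birds remain triggers takeoff and, shortly after, calls OverlapTimeActor on the DeliveryGuy player.
; The player's seeds dispatcher, gated to fire only inside Box1, triggers the same takeoff without that call and sets FlightAway, disabling the Box response.
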(event `self.Box.OnComponentBeginOverlap`
  (params (OverlappedComponent :type "PrimitiveComponent Object Reference") (OtherActor :type "Actor Object Reference") (OtherComp :type "PrimitiveComponent Object Reference") (OtherBodyIndex :type Integer) (bFromSweep :type Boolean) (SweepResult :type "HitResult Structure (by ref)"))
  (bind _paperflipbook (`self.PaperFlipbook`))
  (bind _returnvalue (`PaperFlipbookComponent.GetFlipbook` _paperflipbook))
  (cast `/Game/DeliveryGuy_BP/Blueprints/DeliveryGuy` OtherActor)
  (if (not (`self.FlightAway`))
    (`/Engine/EditorBlueprintResources/StandardMacros.DoOnce` false
      (:`Completed`
        (`|ExecutionSequence`
          (:`then_0`
            (`PaperFlipbookComponent.SetFlipbook` _paperflipbook "/Game/Flipbooks/Environment/golubi_vzlet_Flipbook.golubi_vzlet_Flipbook" :!label _label)
            (`PaperFlipbookComponent.PlayFromStart` (`self.PaperFlipbook`))
            (`PaperFlipbookComponent.PlayFromStart` _paperflipbook)
            (`KismetSystemLibrary.Delay` (* (/ 1.0 (`PaperFlipbook.FramesPerSecond` _returnvalue)) (`KismetMathLibrary.Conv_IntToDouble` (- (`PaperFlipbook.GetNumFrames` _returnvalue) 1))))
            (`self.SetActorHiddenInGame` true))
          (:`then_1`
            (`KismetSystemLibrary.Delay` 0.2)
            (bind _asdelivery_guy (cast `/Game/DeliveryGuy_BP/Blueprints/DeliveryGuy` (`GameplayStatics.GetPlayerCharacter` 0)))
            (`/Game/DeliveryGuy_BP/Blueprints/DeliveryGuy.OverlapTimeActor` _asdelivery_guy 10.0)))))))

(event `self.ReceiveBeginPlay`
  (bind _asdelivery_guy (cast `/Game/DeliveryGuy_BP/Blueprints/DeliveryGuy` (`GameplayStatics.GetPlayerCharacter` 0)))
  (add `/Game/DeliveryGuy_BP/Blueprints/DeliveryGuy.Seeds_Disp` _asdelivery_guy (delegate `DeliveryGuy_Seeds`)))

(event `DeliveryGuy_Seeds`
  (`/Engine/EditorBlueprintResources/StandardMacros.Gate` true :!label _label_2
    (:`Exit`
      (`/Engine/EditorBlueprintResources/StandardMacros.DoOnce` false
        (:`Completed`
          (`|ExecutionSequence`
            (:`then_0`
              (goto _label))
            (:`then_1`
              (set `self.FlightAway` true))))))))

(event `self.Box1.OnComponentBeginOverlap`
  (params (OverlappedComponent :type "PrimitiveComponent Object Reference") (OtherActor :type "Actor Object Reference") (OtherComp :type "PrimitiveComponent Object Reference") (OtherBodyIndex :type Integer) (bFromSweep :type Boolean) (SweepResult :type "HitResult Structure (by ref)"))
  (cast `/Game/DeliveryGuy_BP/Blueprints/DeliveryGuy` OtherActor)
  (goto _label_2 :!via `Open`))

(event `self.Box1.OnComponentEndOverlap`
  (params (OverlappedComponent :type "PrimitiveComponent Object Reference") (OtherActor :type "Actor Object Reference") (OtherComp :type "PrimitiveComponent Object Reference") (OtherBodyIndex :type Integer))
  (cast `/Game/DeliveryGuy_BP/Blueprints/DeliveryGuy` OtherActor)
  (goto _label_2 :!via `Close`))

(fn `UserConstructionScript`)
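; Angry transformer hazard that periodically spawns a Lightning actor and penalizes a DeliveryGuy player caught in its box.
; A looping delay spawns and starts each lightning, passing it the play count and timing.
; Each strike opens a Tick-driven gate for a short window to check box overlaps.
; A DoOnce, reset each cycle, limits the OverlapTimeActor call on the player to once per strike.
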(event `self.ReceiveBeginPlay`
  (bind _delaybetweenlighnings (`self.DelayBetweenLighnings`))
  (`KismetSystemLibrary.Delay` (+ (`self.DelayToLightAgain`) (`self.DelayBetweenLighnings`)) :!label _label)
  (`|ExecutionSequence`
    (:`then_0`
      (bind _returnvalue (`|SpawnActorFromClass` "/Game/Environment_BP/ANGRYTRANSFORMATOR/Lightning.Lightning_C" (`SceneComponent.K2_GetComponentToWorld` (`self.Scene`)) "Undefined" "OverrideRootScale" null (`self.TimesToPlay`) _delaybetweenlighnings null))
      (`|ExecutionSequence`
        (:`then_0`
          (`/Game/Environment_BP/ANGRYTRANSFORMATOR/Lightning.StartLightning` _returnvalue)
          (`|ExecutionSequence`
            (:`then_0`
              (goto _label))
            (:`then_1`
              (`KismetSystemLibrary.Delay` _delaybetweenlighnings)
              (goto _label_2 :!via `Close`))))
        (:`then_1`
          (goto _label_2 :!via `Open`))))
    (:`then_1`
      (goto _label_3 :!via `Reset`))))

(event `self.ReceiveTick`
  (params (DeltaSeconds :type "Float (single-precision)"))
  (`/Engine/EditorBlueprintResources/StandardMacros.Gate` true :!label _label_2
    (:`Exit`
      (bind _asdelivery_guy (cast `/Game/DeliveryGuy_BP/Blueprints/DeliveryGuy` (`GameplayStatics.GetPlayerCharacter` 0)))
      (if (!= (`KismetArrayLibrary.Array_Find` (`PrimitiveComponent.GetOverlappingActors` (`self.Box`) "/Game/DeliveryGuy_BP/Blueprints/DeliveryGuy.DeliveryGuy_C") _asdelivery_guy) -1)
        (`/Engine/EditorBlueprintResources/StandardMacros.DoOnce` false :!label _label_3
          (:`Completed`
            (`/Game/DeliveryGuy_BP/Blueprints/DeliveryGuy.OverlapTimeActor` _asdelivery_guy 10.0)))))))

(fn `UserConstructionScript`)
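; Office environment actor that reveals its interior while the DeliveryGuy player overlaps its Box trigger.
; Begin overlap calls Opened, which shows the table and wall sprites, hides the window and shifts frames and window along Y.
; End overlap and BeginPlay call Closed to reverse this.
; Tick and GetDistance only cast the player; their distance logic is unwired.
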(event `self.ReceiveBeginPlay`
  (`self.Closed`))

(event `self.ReceiveTick`
  (params (DeltaSeconds :type "Float (single-precision)"))
  (bind _asdelivery_guy (cast `/Game/DeliveryGuy_BP/Blueprints/DeliveryGuy` (`GameplayStatics.GetPlayerCharacter` 0))))

(event `self.Box.OnComponentBeginOverlap`
  (params (OverlappedComponent :type "PrimitiveComponent Object Reference") (OtherActor :type "Actor Object Reference") (OtherComp :type "PrimitiveComponent Object Reference") (OtherBodyIndex :type Integer) (bFromSweep :type Boolean) (SweepResult :type "HitResult Structure (by ref)"))
  (cast `/Game/DeliveryGuy_BP/Blueprints/DeliveryGuy` OtherActor)
  (`SceneComponent.SetHiddenInGame` (`self.Window`) true false)
  (`self.Opened`))

(event `self.Box.OnComponentEndOverlap`
  (params (OverlappedComponent :type "PrimitiveComponent Object Reference") (OtherActor :type "Actor Object Reference") (OtherComp :type "PrimitiveComponent Object Reference") (OtherBodyIndex :type Integer))
  (cast `/Game/DeliveryGuy_BP/Blueprints/DeliveryGuy` OtherActor)
  (`SceneComponent.SetHiddenInGame` (`self.Window`) false false)
  (`self.Closed`))

(fn `Closed`
  (`|ExecutionSequence`
    (:`then_0`
      (`SceneComponent.SetHiddenInGame` (`self.table_white_Sprite1`) true false)
      (`SceneComponent.SetHiddenInGame` (`self.table_white_Sprite`) true false)
      (`SceneComponent.SetHiddenInGame` (`self.Stana_white_right`) true false)
      (`SceneComponent.SetHiddenInGame` (`self.Stana_white_left`) true false)
      (`SceneComponent.SetHiddenInGame` (`self.Window`) false false))
    (:`then_1`
      (`SceneComponent.K2_SetRelativeLocation` (`self.Frames`) (0.0 -79.0 241.0) false false)
      (`SceneComponent.K2_SetRelativeLocation` (`self.Window`) (0.0 -79.0 241.0) false false))))

(fn `GetDistance`
  (bind _asdelivery_guy (cast `/Game/DeliveryGuy_BP/Blueprints/DeliveryGuy` (`GameplayStatics.GetPlayerCharacter` 0))))

(fn `Opened`
  (`|ExecutionSequence`
    (:`then_0`
      (`SceneComponent.SetHiddenInGame` (`self.table_white_Sprite1`) false false)
      (`SceneComponent.SetHiddenInGame` (`self.table_white_Sprite`) false false)
      (`SceneComponent.SetHiddenInGame` (`self.Stana_white_right`) false false)
      (`SceneComponent.SetHiddenInGame` (`self.Stana_white_left`) false false)
      (`SceneComponent.SetHiddenInGame` (`self.Window`) true false))
    (:`then_1`
      (`SceneComponent.K2_SetRelativeLocation` (`self.Frames`) (0.0 135.0 241.0) false false)
      (`SceneComponent.K2_SetRelativeLocation` (`self.Window`) (0.0 135.0 241.0) false false))))

(fn `UserConstructionScript`)
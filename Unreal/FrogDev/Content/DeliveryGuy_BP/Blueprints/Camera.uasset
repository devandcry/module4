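; Camera actor for the DeliveryGuy character that follows it along X and sits at discrete height lines taken from placed Height actors.
; Construction caches those actors and their Z values; BeginPlay positions the camera, registers it with the controller and attaches it to the character, while Tick holds an X offset.
; Guarded timelines ease Z to the selected line and realign X, though line selection only matches exact height equality.
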(event `self.ReceiveBeginPlay`
  (bind (_returnvalue_x _returnvalue_y) (`KismetMathLibrary.BreakVector` (+ (`self.K2_GetActorLocation` (`self.CharReference`)) (600.0 0.0 300.0))))
  ;[1 1 1] Beginplay
  (bind _asdelivery_guy (cast `/Game/DeliveryGuy_BP/Blueprints/DeliveryGuy` (`GameplayStatics.GetPlayerCharacter` 0)))
  (set `self.CharReference` _asdelivery_guy)
  (set `self.CurrentLine` (`|GetArrayItem` (`self.ZLines`)))
  (bind _nearestline (`self.CheckTheNearestLine`))
  (set `self.CurrentLine` _nearestline)
  (bind _nearestline_2 (`self.CheckTheNearestLine`))
  (`self.K2_SetActorLocation` (`KismetMathLibrary.MakeVector` _returnvalue_x _returnvalue_y _nearestline_2))
  (bind _asdelivery_guy_controller (cast `/Game/DeliveryGuy_BP/Blueprints/DeliveryGuyController` (`GameplayStatics.GetPlayerController` 0)))
  (`/Game/DeliveryGuy_BP/Blueprints/DeliveryGuyController.SetUpMyCam` _asdelivery_guy_controller self)
  (`self.K2_AttachToComponent` (`/Game/DeliveryGuy_BP/Blueprints/DeliveryGuy.SceneLeft` (`self.CharReference`)) "None" "KeepWorld" "KeepWorld" "SnapToTarget" false))

(event `self.ReceiveTick`
  (params (DeltaSeconds :type "Float (single-precision)"))
  (bind (_returnvalue_x _returnvalue_y _returnvalue_z) (`KismetMathLibrary.BreakVector` (`self.K2_GetActorLocation`)))
  (bind _returnvalue_x_2 (`KismetMathLibrary.BreakVector` (`self.K2_GetActorLocation` (`self.CharReference`))))
  ;[1 1 1] Tick -- updateLocation
  (`|ExecutionSequence`
    (:`then_0`
      (`self.K2_SetActorLocation` (`KismetMathLibrary.MakeVector` (+ _returnvalue_x_2 700.0) _returnvalue_y _returnvalue_z)))))

(event `ChangeZView`
  ;[1 1 1] PlaneChanging-Final
  (if (`self.CanDoTimeline?`)
    (set `self.CanDoTimeline?` false)
    (set `self.ZValueMoveTo` (`self.NearestLineToCharacter`))
    (`KismetSystemLibrary.PrintString` "Hello")
    (bind (_direction _newtrack_0) (`Timeline|ChangeNearestLine` :!via `PlayFromStart`)
      (:`Update`
        (`self.K2_SetActorLocation` (`KismetMathLibrary.MakeVector` (.x (`self.K2_GetActorLocation`)) (.y (`self.K2_GetActorLocation`)) (`KismetMathLibrary.Lerp` (`self.CurrentLine`) (`self.ZValueMoveTo`) _newtrack_0))))
      (:`Finished`
        (set `self.CanDoTimeline?` true)
        (set `self.CurrentLine` (`self.ZValueMoveTo`))))))

(event `AlignmentToChar`
  (bind (_returnvalue_x _returnvalue_y _returnvalue_z) (`KismetMathLibrary.BreakVector` (`self.K2_GetActorLocation`)))
  (bind _returnvalue_x_2 (`KismetMathLibrary.BreakVector` (`self.K2_GetActorLocation` (`self.CharReference`))))
  ;[1 1 1] Alignment to Char
  (if (`self.CanDoAlignment?`)
    (set `self.CanDoAlignment?` false)
    (bind (_direction _newtrack_0) (`Timeline|Timeline_0` :!via `PlayFromStart`)
      (:`Update`
        (`self.K2_SetActorLocation` (`KismetMathLibrary.MakeVector` (`KismetMathLibrary.Lerp` _returnvalue_x (+ _returnvalue_x_2 300.0) _newtrack_0) _returnvalue_y _returnvalue_z)))
      (:`Finished`
        (set `self.CanDoAlignment?` true)
        (set `self.CharPositioniswrong` false)))))

(fn `CheckTheNearestLine`
  (returns (NearestLine :type "Float (double-precision)"))
  (locals (LocalFloat :type "Float (double-precision)") (`First Action?` :type Boolean :default true) (LocalActor :type "/Game/DeliveryGuy_BP/Blueprints/CharacterLevellings/Height Object Reference"))
  (bind _localactor (`local.LocalActor`))
  (bind (_returnvalue_x _returnvalue_y _returnvalue_z) (`KismetMathLibrary.BreakVector` (`self.K2_GetActorLocation` _localactor)))
  (bind (_returnvalue_x_2 _returnvalue_y_2 _returnvalue_z_2) (`KismetMathLibrary.BreakVector` (`self.K2_GetActorLocation` (`self.CharReference`))))
  (bind _returnvalue (- _returnvalue_z_2 -100.0))
  (for _array_element (`self.Zactors`)
    (bind (_returnvalue_x_3 _returnvalue_y_3 _returnvalue_z_3) (`KismetMathLibrary.BreakVector` (`SceneComponent.K2_GetComponentLocation` (`/Game/DeliveryGuy_BP/Blueprints/CharacterLevellings/Height.SphereZ+` _array_element))))
    (bind (_returnvalue_x_4 _returnvalue_y_4 _returnvalue_z_4) (`KismetMathLibrary.BreakVector` (`SceneComponent.K2_GetComponentLocation` (`/Game/DeliveryGuy_BP/Blueprints/CharacterLevellings/Height.SphereZ-` _array_element))))
    (if (and (<= _returnvalue _returnvalue_z_3) (>= _returnvalue _returnvalue_z_4))
      (set `local.LocalActor` _array_element)))
  (bind _output_get (set `self.NearestHeightActor` _localactor))
  (set `/Game/DeliveryGuy_BP/Blueprints/DeliveryGuy.CurrentHeightActor` _output_get (`self.CharReference`))
  (bind _output_get_2 (set `self.NearestLineToCharacter` _returnvalue_z))
  (return _output_get_2))

(fn `Floatpos`
  (params (Float :type "Float (double-precision)"))
  (returns (Output :type "Float (double-precision)"))
  (if (>= Float 0.0)
    (return Float)
    (else
      (return (* Float -1.0)))))

(fn `UserConstructionScript`
  (`KismetArrayLibrary.Array_Clear` (`self.ZLines`))
  (`KismetArrayLibrary.Array_Clear` (`self.Zactors`))
  (bind _outactors (`GameplayStatics.GetAllActorsOfClass` "/Game/DeliveryGuy_BP/Blueprints/CharacterLevellings/Height.Height_C"))
  (for (_array_element _array_index) _outactors
    (bind (_returnvalue_x _returnvalue_y _returnvalue_z) (`KismetMathLibrary.BreakVector` (`self.K2_GetActorLocation` _array_element)))
    (`KismetArrayLibrary.Array_Set` (`self.ZLines`) _array_index _returnvalue_z true)
    (`KismetArrayLibrary.Array_Set` (`self.Zactors`) _array_index _array_element true)))
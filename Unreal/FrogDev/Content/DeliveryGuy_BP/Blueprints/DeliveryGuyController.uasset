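; DeliveryGuyController turns touch swipes into Jump and Slide actions on the DeliveryGuy player character.
; A press records the start point and opens a gate that Tick polls until the finger travels past SwipeThreshold.
; The speed-scaled vertical delta triggers Jump for a sufficient upward swipe, otherwise Slide, then tracking restarts from the current point.
; Release closes the gate and prints a tap or swipe debug label.
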(event `self.ReceiveBeginPlay`
  (bind _asdelivery_guy (cast `/Game/DeliveryGuy_BP/Blueprints/DeliveryGuy` (`GameplayStatics.GetPlayerCharacter` 0)))
  (set `self.CharReference` _asdelivery_guy))

(event `self.ReceiveTick`
  (params (DeltaSeconds :type "Float (single-precision)"))
  (bind (_touchstart_x _touchstart_y) (`KismetMathLibrary.BreakVector2D` (`self.TouchStart`)))
  (bind _charreference (`self.CharReference`))
  (bind (_locationx _locationy) (`self.GetInputTouchState` (`GameplayStatics.GetPlayerController` 0) "Touch1"))
  (bind _returnvalue (`KismetMathLibrary.MakeVector2D` _locationx _locationy))
  (`/Engine/EditorBlueprintResources/StandardMacros.Gate` true :!label _label
    (:`Exit`
      (if (>= (`KismetMathLibrary.VSize2D` (- _returnvalue (stale `StartAgain` _output_get))) (`self.SwipeThreshold`))
        (set `self.TouchStartLoc` (10000.0 10000.0))
        (set `self.TouchPriorLoc` _returnvalue)
        (bind _output_get (set `self.YMove` (* (- _touchstart_y (`.Y` (`KismetMathLibrary.BreakVector2D` _returnvalue))) (`self.SwipeSpeed`))))
        (`KismetSystemLibrary.PrintString` (`KismetStringLibrary.Conv_DoubleToString` _output_get))
        (if (>= _output_get 10.0)
          (`Character.Jump` _charreference)
          (else
            (`/Game/DeliveryGuy_BP/Blueprints/DeliveryGuy.Slide` _charreference)))
        (`self.StartAgain`)))))

(event `StartAgain`
  (bind (_locationx _locationy) (`self.GetInputTouchState` (`GameplayStatics.GetPlayerController` 0) "Touch1"))
  (bind _returnvalue (`KismetMathLibrary.MakeVector2D` _locationx _locationy))
  (set `self.TouchStart` _returnvalue :!label _label_2)
  (bind _output_get (set `self.TouchStartLoc` _returnvalue))
  (set `self.TouchPriorLoc` _output_get)
  (goto _label :!via `Open`))

(event `InputAction|Touch Finger 1`
  (params (Key :type "Key Structure"))
  (:`Pressed`
    (goto _label_2))
  (:`Released`
    (`|ExecutionSequence`
      (:`then_0`
        (goto _label :!via `Close`))
      (:`then_1`
        (if (== (`self.TouchStartLoc`) (`self.TouchPriorLoc`))
          (`KismetSystemLibrary.PrintString` "TAP")
          (elif (>= (`self.YMove`) 10.0)
            (`KismetSystemLibrary.PrintString` "SwipeUP")
            (else
              (`KismetSystemLibrary.PrintString` "SwipeDown"))))))))

(fn `UserConstructionScript`)
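; Height is a numbered line marker actor that follows the player DeliveryGuy along X while keeping its own Y and Z.
; Its construction script numbers it by how many Height actors sit lower, shows "Line" plus that number, and copies Reboot to all instances.
; It also offsets SphereZ vertically and, when Number is above zero, stores the actor numbered one higher as PreviousHeightActor; the spacing snap using it is disconnected.
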(event `self.ReceiveTick`
  (params (DeltaSeconds :type "Float (single-precision)"))
  (bind (_returnvalue_x _returnvalue_y _returnvalue_z) (`KismetMathLibrary.BreakVector` (`self.K2_GetActorLocation`)))
  (bind _asdelivery_guy (cast `/Game/DeliveryGuy_BP/Blueprints/DeliveryGuy` (`GameplayStatics.GetPlayerCharacter` 0)))
  (bind _returnvalue_x_2 (`KismetMathLibrary.BreakVector` (`self.K2_GetActorLocation` _asdelivery_guy)))
  (`self.K2_SetActorLocation` (`KismetMathLibrary.MakeVector` _returnvalue_x_2 _returnvalue_y _returnvalue_z)))

(fn `UserConstructionScript`
  (bind (_returnvalue_x _returnvalue_y _returnvalue_z) (`KismetMathLibrary.BreakVector` (`self.K2_GetActorLocation`)))
  ;[1 1 1] Просто настройка самих акторов, ничего особо важного для кода нет
  (`|ExecutionSequence`
    (:`then_0`
      ;;[1 1 1] Number and text
      (set `self.Number` 0)
      (bind _outactors (`GameplayStatics.GetAllActorsOfClass` "Height_C"))
      (for _array_element _outactors
        (set `/Game/DeliveryGuy_BP/Blueprints/CharacterLevellings/Height.reboot` (`self.reboot`) _array_element))
      (bind _outactors_2 (`GameplayStatics.GetAllActorsOfClass` "Height_C"))
      (for _array_element_2 _outactors_2
        (bind (_returnvalue_x_2 _returnvalue_y_2 _returnvalue_z_2) (`KismetMathLibrary.BreakVector` (`self.K2_GetActorLocation` _array_element_2)))
        (if (> _returnvalue_z _returnvalue_z_2)
          (set `self.Number` (+ (`self.Number`) 1))))
      (`TextRenderComponent.K2_SetText` (`self.TextRender`) (`KismetTextLibrary.Conv_StringToText` (`KismetStringLibrary.Concat_StrStr` "Line" (`KismetStringLibrary.Conv_IntToString` (`self.Number`))))))
    (:`then_1`
      ;;[1 1 1] SpheresRelativeLoc
      (`SceneComponent.K2_SetWorldLocation` (`self.SphereZ+`) (+ (`self.K2_GetActorLocation`) (`KismetMathLibrary.MakeVector` 0.0 0.0 (`self.DistanceBetweenRootAndSphereZ+`))) false false)
      (`SceneComponent.K2_SetWorldLocation` (`self.SphereZ-`) (- (`self.K2_GetActorLocation`) (`KismetMathLibrary.MakeVector` 0.0 0.0 (`self.DistanceBetweenRootAndSphereZ-`))) false false))
    (:`then_2`
      (if (> (`self.Number`) 0)
        (bind _outactors_3 (`GameplayStatics.GetAllActorsOfClass` "Height_C"))
        (for _array_element_3 _outactors_3
          (if (== (- (`/Game/DeliveryGuy_BP/Blueprints/CharacterLevellings/Height.Number` _array_element_3) 1) (`self.Number`))
            (set `self.PreviousHeightActor` _array_element_3)
            (break)))))))
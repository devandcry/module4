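; Main menu shop actor that appears with its map region and opens the shop screen from its button.
; It starts hidden and toggles visibility through open and close events bound on its Region reference.
; Its widget component's Shop_Button triggers creation of a Shop_Widget in the viewport, only while the MainMenuController has no valid CurrentLvl.
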(event `self.ReceiveBeginPlay`
  (`self.SetActorHiddenInGame` true)
  (`|ExecutionSequence`
    (:`then_0`
      (bind _asshop_button (cast `/Game/MainMenu/Shop/Shop_Button` (`WidgetComponent.GetUserWidgetObject` (`self.Widget`))))
      (set `self.ButtonRef` _asshop_button)
      (add `/Game/MainMenu/Shop/Shop_Button.Open` _asshop_button (delegate `OpenWidget`))
      (bind _asmain_menu_controller (cast `/Game/MainMenu/MainMenuController` (`GameplayStatics.GetPlayerController` 0)))
      (set `self.ControllerRef` _asmain_menu_controller))
    (:`then_1`
      (bind _asregion (cast `/Game/MainMenu/Region` (`self.MyRegion`)))
      (add `/Game/MainMenu/Region.Open` _asregion (delegate `Unhide`))
      (add `/Game/MainMenu/Region.Close` _asregion (delegate `HideEvent`)))))

(event `Unhide`
  ;[1 1 1] Скрытие\появление
  (`self.SetActorHiddenInGame` false))

(event `HideEvent`
  ;[1 1 1] Скрытие\появление
  (`self.SetActorHiddenInGame` true))

(event `OpenWidget`
  (if (not (`KismetSystemLibrary.IsValid` (`/Game/MainMenu/MainMenuController.CurrentLvl` (`self.ControllerRef`))))
    (bind _returnvalue (`|CreateWidget` "/Game/MainMenu/Shop/Shop_Widget.Shop_Widget_C"))
    (set `self.WidgetRef` _returnvalue)
    (`UserWidget.AddToViewport` _returnvalue 0)))

(fn `UserConstructionScript`)
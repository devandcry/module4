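; Main-menu level marker actor that stays hidden until its linked Region opens, then shows a Pointer widget for selecting that level.
; Clicking toggles between zooming the MainMenuController camera in and returning it to its previous position.
; Zooming in disables swiping, swaps to the Address widget, plays a sound and opens a level-info widget with map, reputation and money data.
; Closing the region hides the marker and resets any open selection.
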(event `self.ReceiveBeginPlay`
  (`self.SetActorHiddenInGame` true)
  (`|ExecutionSequence`
    (:`then_0`
      (bind _aspointer (cast `/Game/MainMenu/Levels/Pointer` (`WidgetComponent.GetUserWidgetObject` (`self.Widget`))))
      (set `self.WidgetReference` _aspointer)
      (add `/Game/MainMenu/Levels/Pointer.FirstButtonClicked` _aspointer (delegate `StartTimeline`))
      (`/Game/MainMenu/Levels/Pointer.SetMyBP` _aspointer null)
      (bind _asaddress (cast `/Game/MainMenu/Levels/Address` (`WidgetComponent.GetUserWidgetObject` (`self.Widget2`))))
      (`/Game/MainMenu/Levels/Address.SetText` _asaddress (`self.Address`))
      (add `/Game/MainMenu/Levels/Address.Click` _asaddress (delegate `Click`)))
    (:`then_1`
      (bind _asregion (cast `/Game/MainMenu/Region` (`self.MyRegion`)))
      (add `/Game/MainMenu/Region.Open` _asregion (delegate `OpenEvent`))
      (add `/Game/MainMenu/Region.Close` _asregion (delegate `CloseEvent`))
      (bind _asmain_menu_controller (cast `/Game/MainMenu/MainMenuController` (`GameplayStatics.GetPlayerController` 0)))
      (set `self.ControllerReference` _asmain_menu_controller))))

(event `OpenEvent`
  (`self.SetActorHiddenInGame` false))

(event `StartTimeline`
  (bind _controllerreference (`self.ControllerReference`))
  (bind _audiocurvesource (`self.AudioCurveSource`))
  (if (`self.Clicked First Time?`) :!label _label
    (set `self.PreviousPlace` (`self.K2_GetActorLocation` (`/Game/MainMenu/MainMenuController.MyCamera` (`self.ControllerReference`))))
    (`/Game/MainMenu/MainMenuController.TimeLineEventZoom` _controllerreference (- (`self.K2_GetActorLocation`) (50.0 0.0 0.0)) false)
    (set `/Game/MainMenu/MainMenuController.CanSwipe?` false (`self.ControllerReference`))
    (`SceneComponent.SetHiddenInGame` (`self.Widget`) true false)
    (`SceneComponent.SetHiddenInGame` (`self.Widget2`) false false)
    (bind _returnvalue (`|CreateWidget` "/Game/MainMenu/Levels/OpenLevelWidget.OpenLevelWidget_C"))
    (set `self.OpenLevelWidget` _returnvalue)
    (`/Game/MainMenu/Levels/OpenLevelWidget.EventOpen` _returnvalue (`self.MapName`) (`self.WidgetText`) (`self.LevelName`) (`self.GivenReputation`) (`self.GivenMoney`))
    (`UserWidget.AddToViewport` (`self.OpenLevelWidget`) 0)
    (set `self.Clicked First Time?` false)
    (`AudioComponent.SetSound` (`self.AudioCurveSource`) (`self.Sound`))
    (`AudioComponent.Play` _audiocurvesource 0.0)
    (else
      (`/Game/MainMenu/MainMenuController.TimeLineEventZoom` _controllerreference (`self.PreviousPlace`) false)
      (`SceneComponent.SetHiddenInGame` (`self.Widget`) false false)
      (`SceneComponent.SetHiddenInGame` (`self.Widget2`) true false)
      (`Widget.RemoveFromParent` (`self.OpenLevelWidget`))
      (set `self.Clicked First Time?` true)
      (set `self.MultiplySound` -300.0)
      (`AudioComponent.Stop` _audiocurvesource :!label _label_2))))

(event `Click`
  (goto _label))

(event `CloseEvent`
  (`self.SetActorHiddenInGame` true)
  (if (not (`self.Clicked First Time?`))
    (`SceneComponent.SetHiddenInGame` (`self.Widget`) false false)
    (`SceneComponent.SetHiddenInGame` (`self.Widget2`) true false)
    (`Widget.RemoveFromParent` (`self.OpenLevelWidget`))
    (set `self.Clicked First Time?` true)
    (set `/Game/MainMenu/MainMenuController.CanSwipe?` true (`self.ControllerReference`))
    (set `self.MultiplySound` -300.0)
    (goto _label_2)))

(fn `UserConstructionScript`
  (`TextRenderComponent.K2_SetText` (`self.TextRender`) (`self.viewportLevelName`)))